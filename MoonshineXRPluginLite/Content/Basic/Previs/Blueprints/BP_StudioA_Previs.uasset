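; Previs actor for Studio A, an LED stage with floor and M, L, R and T LED meshes.
; The construction script applies hide-in-game flags, individually or all at once, and switches M, L and R between debug and grid materials.
; On BeginPlay, a valid PrevisCamera triggers the camera info widget and a blended view switch to that camera.
; GetCamInfo returns its name, filmback and focal length.
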(event `self.ReceiveBeginPlay`
  (`/Engine/EditorBlueprintResources/StandardMacros.IsValid` (`self.PrevisCamera`)
    (:`Is Valid`
      (`|ExecutionSequence`
        (:`then_0`
          (bind _returnvalue (`|GenericCreateObject` "/MoonshineXRPlugin/Basic/Previs/Blueprints/EUW_Cam_Info.EUW_Cam_Info_C"))
          (`UserWidget.AddToViewport` _returnvalue 0))
        (:`then_1`
          (`PlayerController.SetViewTargetWithBlend` (`GameplayStatics.GetPlayerController` 0) (`self.PrevisCamera`) 0.5 "VTBlend_Linear" 0.0 false))
        (:`then_2`
          (`self.GetCamInfo`))))))

(fn `GetCamInfo`
  (returns (`Cam Name` :type String) (Filmback :type String) (SensorSize :type "CameraFilmbackSettings Structure") (`Focal Length` :type "Float (single-precision)"))
  (bind _previscamera (`self.PrevisCamera`))
  (bind _returnvalue (`CineCameraActor.GetCineCameraComponent` _previscamera))
  (`/Engine/EditorBlueprintResources/StandardMacros.IsValid` (`self.PrevisCamera`)
    (:`Is Valid`
      (return (`KismetSystemLibrary.GetDisplayName` _previscamera) (`CineCameraComponent.GetFilmbackPresetName` _returnvalue) (`CineCameraComponent.Filmback` _returnvalue) (`CineCameraComponent.CurrentFocalLength` _returnvalue)))))

(fn `ToggleLEDMaterial`
  (params (bShowDebugMaterial :type Boolean) (LED :type "PrimitiveComponent Object Reference") (DebugMaterial :type "MaterialInterface Object Reference") (GridMaterial :type "MaterialInterface Object Reference"))
  (if bShowDebugMaterial
    (`PrimitiveComponent.SetMaterial` LED 0 DebugMaterial)
    (else
      (`PrimitiveComponent.SetMaterial` LED 0 GridMaterial))))

(fn `UserConstructionScript`
  (`|ExecutionSequence`
    (:`then_0`
      (if (`self.bHideAll`)
        (`SceneComponent.SetHiddenInGame` (`self.DefaultSceneRoot`) (`self.bHideAll`) true)
        (else
          (`|ExecutionSequence`
            (:`then_0`
              (`SceneComponent.SetHiddenInGame` (`self.LEDfloor`) (`self.bHideStage`) true))
            (:`then_1`
              (`SceneComponent.SetHiddenInGame` (`self.SM_A_LED_M`) (`self.bHideLED_M`) false)
              (`SceneComponent.SetHiddenInGame` (`self.SM_A_LED_L`) (`self.bHideLED_L`) false)
              (`SceneComponent.SetHiddenInGame` (`self.SM_A_LED_R`) (`self.bHideLED_R`) false)
              (`SceneComponent.SetHiddenInGame` (`self.SM_A_LED_T`) (`self.bHideLED_T`) false))))))
    (:`then_1`
      (`self.ToggleLEDMaterial` (`self.bShowDebugMaterial_M`) (`self.SM_A_LED_M`) (`self.DebugMaterial_M`) "/MoonshineXRPlugin/Basic/Previs/Assets/StageA/Materials/M_Previs_Grid_M.M_Previs_Grid_M")
      (`self.ToggleLEDMaterial` (`self.bShowDebugMaterial_L`) (`self.SM_A_LED_L`) (`self.DebugMaterial_L`) "/MoonshineXRPlugin/Basic/Previs/Assets/StageA/Materials/M_Previs_Grid_L.M_Previs_Grid_L")
      (`self.ToggleLEDMaterial` (`self.bShowDebugMaterial_R`) (`self.SM_A_LED_R`) (`self.DebugMaterial_R`) "/MoonshineXRPlugin/Basic/Previs/Assets/StageA/Materials/M_Previs_Grid_R.M_Previs_Grid_R"))))