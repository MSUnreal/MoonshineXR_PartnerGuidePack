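; BP_Mask_StudioKH is a mask actor for the StudioKH LED meshes: LEDL, LEDM, LEDR and LEDF.
; Its construction script runs the parent's, then calls BindMaskMaterialParam on each mesh with that mesh's own mask parameter set and a shared ParamName.
; The event graph holds only disabled default events, so all of its own logic runs at construction.
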(fn `UserConstructionScript`
  (`parent.UserConstructionScript`)
  (`self.Bind Mask Material Param` (`self.LED_L`) (`self.L_Material_Param`) (`self.Param_Name`))
  (`self.Bind Mask Material Param` (`self.LED_M`) (`self.M_Material_Param`) (`self.Param_Name`))
  (`self.Bind Mask Material Param` (`self.LED_R`) (`self.R_Material_Param`) (`self.Param_Name`))
  (`self.Bind Mask Material Param` (`self.LED_F`) (`self.F_Material_Param`) (`self.Param_Name`)))